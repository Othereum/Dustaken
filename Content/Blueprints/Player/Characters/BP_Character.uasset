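; Player character Blueprint that creates the HUD and handles the character's death.
; On BeginPlay it adds the HUD widget to the owning player's screen.
; OnKill detaches the active weapon as a physics object, turns off capsule collision and input, ragdolls the mesh and unlinks both cameras from control rotation.
; It then reports the victim and last attacker to the BP_GM game mode.
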(event EventOnKill
  (bind _mesh (Variables|Character|GetMesh))
  (bind _weaponcomponent (Variables|Default|GetWeaponComponent))
  (bind _returnvalue (Class|WeaponComponent|GetActiveWeapon _weaponcomponent))
  (bind _mesh_2 (Variables|/Script/Dustaken.Weapon|GetMesh _returnvalue))
  (Utilities|FlowControl|Sequence
    (:then_0
      (Transformation|DetachFromComponent _mesh_2 "KeepWorld" "KeepWorld" "KeepWorld" true)
      (Physics|SetSimulatePhysics _mesh_2 true)
      (Collision|SetCollisionEnabled _mesh_2 "QueryAndPhysics")
      (Collision|SetCollisionEnabled (Variables|Default|GetCapsuleComponent) "NoCollision")
      (Input|DisableInput 0)
      (Collision|SetCollisionEnabled _mesh "QueryAndPhysics")
      (Physics|SetSimulatePhysics _mesh true)
      (Variables|/Script/Engine.CameraComponent|SetbUsePawnControlRotation (Variables|Default|GetCameraComponent) false)
      (Variables|/Script/Engine.CameraComponent|SetbUsePawnControlRotation (Variables|Default|GetAimCamera) false))
    (:then_1
      (bind _asbp_gm (Utilities|Casting|CastToBP_GM (Game|GetGameMode)))
      (Default|OnPlayerDeath _asbp_gm self (Variables|Default|GetLastHitBy)))))

(event EventBeginPlay
  (bind _asplayer_controller (Utilities|Casting|CastToPlayerController (Pawn|GetController)))
  (bind _returnvalue (UserInterface|CreateWidget "/Game/Blueprints/Player/WidgetBP_HUD.WidgetBP_HUD_C" _asplayer_controller))
  (UserInterface|Viewport|AddtoPlayerScreen _returnvalue))

(fn ConstructionScript)