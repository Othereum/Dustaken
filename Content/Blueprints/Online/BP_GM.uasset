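; Game mode for an online last-player-standing FPS that names joining players sequentially and gives spawned characters an AK47 and an M4.
; On each death it counts living characters; when one or none remains, it broadcasts any winner in Korean and respawns everyone after a short delay.
; Helper functions gather controllers and send client messages by walking player indices until the BP_PC cast fails.
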(event Custom|OnPlayerDeath
  (params (Victim :type BP%20Character%20Object%20Reference) (Attacker :type Controller%20Object%20Reference))
  (bind (_numalive _alivepc) (CallFunction|NumAlive))
  (if (<= _numalive 1)
    (Utilities|FlowControl|Sequence
      (:then_0
        (Utilities|FlowControl|Delay 3.0)
        (for _array_element (CallFunction|GetAllPlayerControllers)
          (Actor|DestroyActor (Pawn|GetControlledPawn _array_element))
          (Class|GameModeBase|RestartPlayer _array_element)))
      (:then_1
        (Utilities|IsValid _alivepc
          (:Is%20Valid
            (CallFunction|BroadcastMsg (Utilities|Text|FormatText "{Name} 님이 이겼어요! 한판 더 달려요옷!!" (Variables|/Game/Blueprints/Player/BP_PC.BP_PC_C|GetPlayerName _alivepc)))))))))

(event EventPostLogin
  (params (NewPlayer :type Player%20Controller%20Object%20Reference))
  (bind _asbp_pc (Utilities|Casting|CastToBP_PC NewPlayer))
  (bind _output_get (Variables|Default|SetPlyIdx (+ (Variables|Default|GetPlyIdx) 1)))
  (Variables|/Game/Blueprints/Player/BP_PC.BP_PC_C|SetPlayerName _asbp_pc (Utilities|Text|FormatText "Player{n}" _output_get)))

(fn ConstructionScript)

(fn SpawnDefaultPawnfor
  (params (NewPlayer :type Controller%20Object%20Reference) (StartSpot :type Actor%20Object%20Reference))
  (bind _returnvalue (|CallParentFunction NewPlayer StartSpot))
  (bind _asfps_character (Utilities|Casting|CastToFpsCharacter _returnvalue))
  (Class|WeaponComponent|Give (Variables|/Script/Dustaken.FpsCharacter|GetWeaponComponent _asfps_character) "/Game/Blueprints/Weapon/BP_AK47.BP_AK47_C")
  (Class|WeaponComponent|Give (Variables|/Script/Dustaken.FpsCharacter|GetWeaponComponent _asfps_character) "/Game/Blueprints/Weapon/BP_M4.BP_M4_C")
  (return _returnvalue))

(fn BroadcastMsg
  (params (Msg :type Text))
  (bind _asbp_pc (Utilities|Casting|CastToBP_PC (Game|GetPlayerController (LocalVariables|GetPlayerIndex)) :!label _label))
  (Default|ClientMsg _asbp_pc Msg)
  (Math|Integer|IncrementInt (LocalVariables|GetPlayerIndex)
    (:%20%20
      (goto _label))))

(fn NumAlive
  (for _array_element (CallFunction|GetAllPlayerControllers)
    (bind _asbp_character (Utilities|Casting|CastToBP_Character (Pawn|GetControlledPawn _array_element)))
    (if (Variables|/Script/Dustaken.FpsCharacter|GetbAlive _asbp_character)
      (Math|Integer|IncrementInt (LocalVariables|GetNum)
        (:%20%20
          (LocalVariables|SetAlive _array_element)))))
  (return (LocalVariables|GetNum) (LocalVariables|GetAlive)))

(fn GetAllPlayerControllers
  (bind _pcarr (LocalVariables|GetPCArr))
  (bind _asbp_pc (Utilities|Casting|CastToBP_PC (Game|GetPlayerController (LocalVariables|GetPlayerIndex)) :!label _label)
    (:then
      (Utilities|Array|Add _pcarr _asbp_pc)
      (Math|Integer|IncrementInt (LocalVariables|GetPlayerIndex)
        (:%20%20
          (goto _label))))
    (:CastFailed
      (return _pcarr))))